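; BP_LightDetector is a light-detection component for the third-person character that displays how brightly lit the player is.
; On begin play it spawns an emissive text actor and starts the inherited thread worker.
; Each tick it shows GetBrightness as a percentage above the player, yawed toward the follow camera.
; Near darkness it turns on the head lamp, recolors the text blue and sets IgnoreBlueColor, reverting when brighter.
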(event EventBeginPlay
  (|CallParentFunction)
  (bind _asthird_person_character (Utilities|Casting|CastToThirdPersonCharacter (Components|GetOwner)))
  (bind _output_get (Variables|Default|SetPlayer _asthird_person_character))
  (bind _returnvalue (Game|SpawnActorfromClass "/Script/Engine.TextRenderActor" (Math|Transform|MakeTransform "0, 0, 0" "0, 0, 0" "1.000000,1.000000,1.000000") "AlwaysSpawn" _output_get _output_get))
  (bind _output_get_2 (Variables|Default|SetTextRenderer _returnvalue))
  (Collision|SetActorEnableCollision _output_get_2 false)
  (Rendering|Components|TextRender|SetXScale (Variables|/Script/Engine.TextRenderActor|GetTextRender _output_get_2) 1.0)
  (Rendering|Components|TextRender|SetYScale (Variables|/Script/Engine.TextRenderActor|GetTextRender _output_get_2) 1.0)
  (Rendering|Components|TextRender|SetTextRenderColor (Variables|/Script/Engine.TextRenderActor|GetTextRender _output_get_2) (Math|Color|MakeColor 128 128 128))
  (Class|TextRenderComponent|SetTextMaterial (Variables|/Script/Engine.TextRenderActor|GetTextRender _output_get_2) "/Game/StealthMeter/DefaultTextMaterialEmissive.DefaultTextMaterialEmissive")
  (Class|LightDetector|StartThreadWorker)
  (Development|PrintString "Thread Worker Started" true true "(R=1.000000,G=0.912126,B=0.000000,A=1.000000)" 5.0))

(event EventTick
  (params (DeltaSeconds :type Float%20%28single-precision%29))
  (bind _textrenderer (Variables|Default|GetTextRenderer))
  (bind _textrenderer_2 (Variables|Default|GetTextRenderer))
  (bind _player (Variables|Default|GetPlayer))
  (bind _player_2 (Variables|Default|GetPlayer))
  (bind _returnvalue (Transformation|GetActorLocation _player_2))
  (bind _textrender (Variables|/Script/Engine.TextRenderActor|GetTextRender _textrenderer))
  (bind _headlamp (Variables|/Game/ThirdPersonCPP/Blueprints/ThirdPersonCharacter.ThirdPersonCharacter_C|GetHeadLamp _player))
  (|CallParentFunction DeltaSeconds)
  (Utilities|IsValid (Variables|Default|GetPlayer)
    (:Is%20Valid
      (Utilities|IsValid _textrenderer_2
        (:Is%20Valid
          (Rendering|Components|TextRender|SetText (Variables|/Script/Engine.TextRenderActor|GetTextRender _textrenderer_2) (Utilities|Text|ToText(String) (Utilities|String|MakeLiteralString (Utilities|String|Append "%" (Utilities|String|ToString(Text) (Utilities|Text|ToText(Float) (* (Class|LightDetector|GetBrightness) 1e+02) "HalfToEven" false true 1 324 0 0))))))
          (Transformation|SetActorLocationAndRotation (Variables|Default|GetTextRenderer) (Math|Vector|MakeVector (.x _returnvalue) (.y _returnvalue) (+ (.z _returnvalue) 7e+01)) (Math|Rotator|MakeRotator 0.0 0.0 (.yaw (Math|Rotator|FindLookatRotation (Transformation|GetActorLocation (Variables|Default|GetTextRenderer)) (Transformation|GetWorldLocation (Variables|/Script/StealthMeterExample.StealthMeterExampleCharacter|GetFollowCamera _player_2))))))
          (if (<= (Class|LightDetector|GetBrightness) 0.05)
            (Variables|Default|SetIgnoreBlueColor true)
            (Rendering|SetVisibility _headlamp true false)
            (Rendering|Components|TextRender|SetTextRenderColor _textrender (Math|Color|MakeColor 128 0 0))
            (else
              (Variables|Default|SetIgnoreBlueColor false)
              (Rendering|SetVisibility _headlamp false false)
              (Rendering|Components|TextRender|SetTextRenderColor _textrender (Math|Color|MakeColor 128 128 128)))))))))